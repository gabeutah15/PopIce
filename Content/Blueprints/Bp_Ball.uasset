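; Brick-breaker ball that moves by projectile movement, bouncing off the paddle and destroying blocks it hits.
; Block hits notify the game mode, destroy the block, add Frenzy manager energy, and randomly spawn a collectible, occasionally with an extra ball.
; Paddle hits add scaled paddle velocity.
; Tick enforces minimum vertical speed and, with OnProjectileStop, tries to restart stalled balls; destructible-brick and overlap logic is disconnected.
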(event OnProjectileStop(ProjectileMovement)
  (params (ImpactResult :type Hit%20Result%20Structure%20%28by%20ref%29))
  (Variables|/Script/Engine.MovementComponent|SetVelocity (Variables|Default|GetProjectileMovement) (Variables|Default|GetInitialVelocity)))

(event OnComponentHit(Sphere)
  (params (HitComponent :type Primitive%20Component%20Object%20Reference) (OtherActor :type Actor%20Object%20Reference) (OtherComp :type Primitive%20Component%20Object%20Reference) (NormalImpulse :type Vector :default "0, 0, 0") (Hit :type Hit%20Result%20Structure%20%28by%20ref%29))
  (bind _projectilemovement (Variables|Default|GetProjectileMovement))
  (bind _frenzymode (Variables|Default|GetFrenzymode))
  (bind _asbp_block (Utilities|Casting|CastToBP_Block OtherActor)
    (:then
      (Utilities|FlowControl|Sequence
        (:then_0
          (Class|BPIBlock|CheckBricks(Message) (Variables|Default|GetREF_Gamemode))
          (Math|Integer|CompareInt (Math|Random|RandomInteger 3) 1
            (:==
              (Game|SpawnActorfromClass "/Game/Blueprints/BP_Collectible.BP_Collectible_C" (Math|Transform|MakeTransform (Transformation|GetActorLocation _asbp_block) "0, 0, 0" "1,1,1") "AlwaysSpawn" 0 0)
              (Math|Integer|CompareInt (Math|Random|RandomInteger 20) 2
                (:==
                  (Game|SpawnActorfromClass "Bp_Ball_C" (Math|Transform|MakeTransform (Math|Vector|MakeVector (.X (Math|Vector|BreakVector (Transformation|GetActorLocation _asbp_block))) 1e+01 (.Z (Math|Vector|BreakVector (Transformation|GetActorLocation _asbp_block)))) "0, 0, 0" "1.600000,1.600000,1.600000") "AdjustIfPossibleButAlwaysSpawn" 0 0))))))
        (:then_1
          (Class|BPIBlock|AddDestroyedBlockLocation(Message) (Variables|Default|GetREF_Gamemode) (Transformation|GetActorLocation _asbp_block)))
        (:then_2
          (Actor|DestroyActor _asbp_block)
          (bind _output_get (Variables|/Game/Blueprints/BP_FrenzyManager.BP_FrenzyManager_C|SetEnergy _frenzymode (+ (Variables|/Game/Blueprints/BP_FrenzyManager.BP_FrenzyManager_C|GetEnergy _frenzymode) 1)))
          (Development|PrintString (Utilities|String|ToString(Integer) _output_get)))))
    (:CastFailed
      (bind _asbp_paddle (Utilities|Casting|CastToBP_Paddle OtherActor))
      (Variables|/Script/Engine.MovementComponent|SetVelocity _projectilemovement (+ (Variables|/Script/Engine.MovementComponent|GetVelocity _projectilemovement) (* (Variables|/Game/Blueprints/BP_Paddle.BP_Paddle_C|GetVelocityPaddle _asbp_paddle) 100)))
      (Development|PrintString (Utilities|String|ToString(Vector) (* (Variables|/Game/Blueprints/BP_Paddle.BP_Paddle_C|GetVelocityPaddle _asbp_paddle) 100))))))

(event EventBeginPlay
  (bind _asbp_gm_block (Utilities|Casting|CastToBP_GM_Block (Game|GetGameMode)))
  (Variables|Default|SetREF_Gamemode _asbp_gm_block)
  (Variables|/Script/Engine.MovementComponent|SetVelocity (Variables|Default|GetProjectileMovement) (Variables|Default|GetInitialVelocity))
  (bind _returnvalue (Actor|GetActorOfClass "/Game/Blueprints/BP_FrenzyManager.BP_FrenzyManager_C"))
  (Variables|Default|SetFrenzymode _returnvalue))

(event EventTick
  (params (DeltaSeconds :type Float%20%28single-precision%29))
  (bind _projectilemovement (Variables|Default|GetProjectileMovement))
  (if (and (< (Math|Float|Absolute(Float) (.x (Variables|/Script/Engine.MovementComponent|GetVelocity _projectilemovement))) 1e+01) (< (Math|Float|Absolute(Float) (.z (Variables|/Script/Engine.MovementComponent|GetVelocity _projectilemovement))) 1e+01)) ; this does not actually work though, balls will still stop\nsometimes and not move again
    (Variables|/Script/Engine.MovementComponent|SetVelocity _projectilemovement "0, 0,1000.000000")
    (elif (and (< (.z (Variables|/Script/Engine.MovementComponent|GetVelocity (Variables|Default|GetProjectileMovement))) 0.0) (> (.z (Variables|/Script/Engine.MovementComponent|GetVelocity (Variables|Default|GetProjectileMovement))) (- 0.0 (Variables|Default|GetMinimumZVelocity)))) ; If Z is negative but not fast enough
      (Variables|/Script/Engine.MovementComponent|SetVelocity (Variables|Default|GetProjectileMovement) (Math|Vector|MakeVector (.x (Variables|/Script/Engine.MovementComponent|GetVelocity (Variables|Default|GetProjectileMovement))) (.y (Variables|/Script/Engine.MovementComponent|GetVelocity (Variables|Default|GetProjectileMovement))) (- 0.0 (Variables|Default|GetMinimumZVelocity)))) ; Set Z to be the minimum negative velocity
      (elif (and (>= (.z (Variables|/Script/Engine.MovementComponent|GetVelocity (Variables|Default|GetProjectileMovement))) 0.0) (< (.z (Variables|/Script/Engine.MovementComponent|GetVelocity (Variables|Default|GetProjectileMovement))) (Variables|Default|GetMinimumZVelocity))) ; If Z is non-negative but not fast enough
        (Variables|/Script/Engine.MovementComponent|SetVelocity (Variables|Default|GetProjectileMovement) (Math|Vector|MakeVector (.x (Variables|/Script/Engine.MovementComponent|GetVelocity (Variables|Default|GetProjectileMovement))) (.y (Variables|/Script/Engine.MovementComponent|GetVelocity (Variables|Default|GetProjectileMovement))) (Variables|Default|GetMinimumZVelocity))) ; Set Z to be the minimum velocity
      ))))

(event Collision|EventActorBeginOverlap
  (params (OtherActor :type Actor%20Object%20Reference)))

(fn ConstructionScript)