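; Game mode for a brick-breaker that tracks lives, coins and remaining blocks, counting BP_Block actors at BeginPlay.
; Losing a life respawns the ball until none remain; running out of lives or blocks pauses into the game-over screen with a result.
; HUD and game-over widgets are reached through BP_GI_Block.
; TwitchMessage maps "coin", "left" and "right" messages to adding a coin or nudging the paddle with sweep.
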(event Custom|EndGame
  (params (ENUM_GameResult :type ENUM_GameResult%20Enum :default "NewEnumerator0"))
  (bind _ref_gameinstance (Variables|Default|GetREF_GameInstance))
  (Default|CallGameOverWBP _ref_gameinstance)
  (Default|SetEndResult (Variables|/Game/Blueprints/BP_GI_Block.BP_GI_Block_C|GetREF_GameOver _ref_gameinstance) ENUM_GameResult)
  (Variables|/Script/Engine.PlayerController|SetbShowMouseCursor (Game|GetPlayerController 0) true)
  (Game|SetGamePaused true))

(event EventBeginPlay
  (Utilities|FlowControl|Sequence
    (:then_0
      (bind _asbp_gi_block (Utilities|Casting|CastToBP_GI_Block (Game|GetGameInstance)))
      (Variables|Default|SetREF_GameInstance _asbp_gi_block))
    (:then_1
      (Variables|Default|SetLives 3)
      (Variables|Default|SetCoins 0))
    (:then_2
      (bind _outactors (Actor|GetAllActorsOfClass "/Game/Blueprints/BP_Block.BP_Block_C"))
      (Variables|Default|SetBlocks (Utilities|Array|Length _outactors)))))

(event EventTwitchMessage
  (params (RawMessage :type String) (Paddle :type BP%20Paddle%20Object%20Reference))
  (if (Utilities|Enum|Equal(Enum) RawMessage "coin")
    (Math|Integer|IncrementInt (Variables|Default|GetCoins)
      (:%20%20
        (Default|CheckCoins (Variables|/Game/Blueprints/BP_GI_Block.BP_GI_Block_C|GetREF_HUD (Variables|Default|GetREF_GameInstance)) (Variables|Default|GetCoins))))
    (elif (Utilities|Enum|Equal(Enum) RawMessage "left")
      (Transformation|AddWorldOffset (Variables|/Script/Engine.Actor|GetRootComponent Paddle) "100.000000, 0, 0" true false)
      (elif (Utilities|Enum|Equal(Enum) RawMessage "right")
        (Transformation|AddWorldOffset (Variables|/Script/Engine.Actor|GetRootComponent Paddle) "-100.000000, 0, 0" true false)))))

(event EventCheckLives
  (Math|Integer|DecrementInt (Variables|Default|GetLives)
    (:%20%20
      (Default|UpdateLives (Variables|/Game/Blueprints/BP_GI_Block.BP_GI_Block_C|GetREF_HUD (Variables|Default|GetREF_GameInstance)) (Variables|Default|GetLives))
      (if (== (Variables|Default|GetLives) 0)
        (CallFunction|EndGame "NewEnumerator1")
        (else
          (Game|SpawnActorfromClass "/Game/Blueprints/Bp_Ball.Bp_Ball_C" (Math|Transform|MakeTransform "0,0.000000,1100.000000" "0, 0, 0" "1,1,1") "Undefined" 0 0))))))

(event EventCheckBricks
  (bind _result (Math|Integer|DecrementInt (Variables|Default|GetBlocks))
    (:%20%20
      (if (== _result 0)
        (CallFunction|EndGame "NewEnumerator0")))))

(event EventStartGame
  (Game|SetGamePaused false)
  (Default|CallHUDWBP (Variables|Default|GetREF_GameInstance)))

(event EventCheckCoins
  (Math|Integer|IncrementInt (Variables|Default|GetCoins)
    (:%20%20
      (Default|CheckCoins (Variables|/Game/Blueprints/BP_GI_Block.BP_GI_Block_C|GetREF_HUD (Variables|Default|GetREF_GameInstance)) (Variables|Default|GetCoins)))))

(fn ConstructionScript)