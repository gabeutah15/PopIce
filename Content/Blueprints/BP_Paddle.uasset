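; BP_Paddle is a player-controlled paddle for a block game that moves along the X axis.
; BeginPlay caches the BP_GM_Block game mode.
; The MoveRight axis, scaled by PaddleSpeed without delta time, sets VelocityPaddle on both itself and the game mode's InitialPaddle.
; The same vector then moves InitialPaddle's root and this paddle's own sprite as swept world offsets.
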(event EventBeginPlay
  (bind _asbp_gm_block (Utilities|Casting|CastToBP_GM_Block (Game|GetGameMode))))

(event Input|AxisEvents|InputAxisMoveRight
  (params (AxisValue :type Float%20%28single-precision%29))
  (bind _paddlespeed (Variables|Default|GetPaddleSpeed))
  (bind _returnvalue (* AxisValue _paddlespeed))
  (bind _returnvalue_2 (* "1.000000, 0, 0" _returnvalue))
  (Variables|BP_Paddle_C|SetVelocityPaddle (Variables|/Game/Blueprints/BP_GM_Block.BP_GM_Block_C|GetInitialPaddle (stale EventBeginPlay _asbp_gm_block)) _returnvalue_2)
  (bind _output_get (Variables|Default|SetVelocityPaddle _returnvalue_2))
  (Transformation|AddWorldOffset (Variables|/Script/Engine.Actor|GetRootComponent (Variables|/Game/Blueprints/BP_GM_Block.BP_GM_Block_C|GetInitialPaddle (stale EventBeginPlay _asbp_gm_block))) _returnvalue_2 true false)
  (Transformation|AddWorldOffset (Variables|Default|GetT_Paddle_D_Sprite) _returnvalue_2 true false))

(fn ConstructionScript)