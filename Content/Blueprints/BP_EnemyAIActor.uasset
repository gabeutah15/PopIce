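; BP_EnemyAIActor is an enemy that slides along the world X axis while periodically firing projectiles.
; A timeline lerps it without sweep between offsets either side of its starting location, restarting from the beginning whenever it finishes.
; A looping timer calls Fire, which waits briefly, spawns a BP_EnemyAIProjectile at the Cone's location, passes it the BP_GM_Block game mode and launches it.
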(event Custom|ResetTimeline
  (bind _newtrack_1 (Timeline|Timeline_0 PlayFromStart) ; some weirdness with where this ends
    (:Update
      (Transformation|SetActorLocation (Math|Vector|Lerp(Vector) (stale EventBeginPlay _output_get) (stale EventBeginPlay _output_get_2) _newtrack_1) false false))
    (:Finished
      (CallFunction|ResetTimeline))))

(event Custom|Fire
  (bind _asbp_gm_block (Utilities|Casting|CastToBP_GM_Block (Game|GetGameMode)))
  (Variables|Default|SetREF_GameMode _asbp_gm_block)
  (Utilities|FlowControl|Delay 2.0)
  (bind _returnvalue (Game|SpawnActorfromClass "/Game/Blueprints/BP_EnemyAIProjectile.BP_EnemyAIProjectile_C" (Math|Conversions|ToTransform(Vector) (Transformation|GetWorldLocation (Variables|Default|GetCone))) "AlwaysSpawn" 0 0))
  (Variables|/Game/Blueprints/BP_EnemyAIProjectile.BP_EnemyAIProjectile_C|SetREF_Gamemode _returnvalue (Variables|Default|GetREF_GameMode))
  (Default|FireProjectile _returnvalue))

(event EventBeginPlay
  (bind _returnvalue (Transformation|GetActorLocation))
  (Utilities|FlowControl|Sequence
    (:then_0
      (bind _output_get (Variables|Default|SetStartPosition (+ _returnvalue "-2500.000000, 0, 0")))
      (bind _output_get_2 (Variables|Default|SetEndPosition (+ _returnvalue "2500.000000, 0, 0")))
      (bind _newtrack_1 (Timeline|Timeline_0 Play) ; some weirdness with where this ends
        (:Update
          (Transformation|SetActorLocation (Math|Vector|Lerp(Vector) _output_get _output_get_2 _newtrack_1) false false))
        (:Finished
          (CallFunction|ResetTimeline))))
    (:then_1
      (Utilities|Time|SetTimerbyEvent (delegate Custom|Fire) 2.0 true))))

(event Collision|EventActorBeginOverlap
  (params (OtherActor :type Actor%20Object%20Reference)))

(event EventTick
  (params (DeltaSeconds :type Float%20%28single-precision%29)))

(fn ConstructionScript)