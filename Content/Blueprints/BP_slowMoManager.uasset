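; BP_slowMoManager toggles slow motion that slows the world while compensating the player pawn.
; ToggleSlowMotion uses a FlipFlop to alternate global time dilation between SlowMotionScale and normal, with a sound for each switch.
; On slowdown, a Delay of SlowMotionScale precedes setting the pawn's CustomTimeDilation to the inverse scale.
; Speeding up restores both dilations immediately.
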(event Custom|ToggleSlowMotion
  (bind _returnvalue (Game|Player|GetPlayerPawn 0))
  (bind _slowmotionscale (Variables|Default|GetslowMotionScale))
  ;[1 1 1] Toggle slow motion: only on environment, not affecting player pawn
  (Utilities|FlowControl|FlipFlop
    (:A
      (Audio|PlaySound2D "/Game/SFX/Slow_Motion_SFX_SlowingDown.Slow_Motion_SFX_SlowingDown" 1.0 1.0 0.0 0 0)
      (Utilities|Time|SetGlobalTimeDilation _slowmotionscale)
      (Utilities|FlowControl|Delay _slowmotionscale)
      (Variables|/Script/Engine.Actor|SetCustomTimeDilation _returnvalue (/ 1.0 _slowmotionscale)))
    (:B
      (Audio|PlaySound2D "/Game/SFX/Slow_Motion_SFX_SpeedingUp.Slow_Motion_SFX_SpeedingUp" 1.0 1.0 0.0 0 0)
      (Utilities|Time|SetGlobalTimeDilation 1.0)
      (Variables|/Script/Engine.Actor|SetCustomTimeDilation _returnvalue 1.0))))

(fn ConstructionScript)