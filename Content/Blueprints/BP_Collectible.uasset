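; BP_Collectible is a short-lived coin pickup that the paddle catches in a block game.
; On BeginPlay it caches the BP_GM_Block game mode and destroys itself after a fixed delay if uncollected.
; Overlapping a BP_Paddle calls CheckCoinsMessage on the game mode and destroys the pickup immediately.
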(event EventBeginPlay
  (Utilities|FlowControl|Sequence
    (:then_0
      (bind _asbp_gm_block (Utilities|Casting|CastToBP_GM_Block (Game|GetGameMode)))
      (Variables|Default|SetREF_GameMode _asbp_gm_block))
    (:then_1
      (Utilities|FlowControl|Delay 5.0)
      (Actor|DestroyActor))))

(event Collision|EventActorBeginOverlap
  (params (OtherActor :type Actor%20Object%20Reference))
  (Utilities|Casting|CastToBP_Paddle OtherActor)
  (Class|BPIBlock|CheckCoins(Message) (Variables|Default|GetREF_GameMode))
  (Actor|DestroyActor))

(fn ConstructionScript)