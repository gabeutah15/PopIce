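; BP_FrenzyManager is an unfinished frenzy manager built around an Energy value and the collision of Bp_Ball actors.
; Tick checks whether Energy has reached a threshold, but the branch leads nowhere.
; A disconnected chain would set every ball's sphere to overlap on a custom trace channel, restore blocking after a delay, then deduct Energy.
; As wired, that frenzy effect never runs.
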(event EventTick
  (params (DeltaSeconds :type Float%20%28single-precision%29))
  (if (>= (Variables|Default|GetEnergy) 15)
    _))

(event Input|KeyboardEvents|NumPadFive
  (params (Key :type Key%20Structure :default "None")))

(fn ConstructionScript)