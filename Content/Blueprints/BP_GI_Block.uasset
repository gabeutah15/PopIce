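; BP_GI_Block, apparently the Game Instance, creates and displays the main menu, HUD and game over widgets.
; Each screen has its own custom event that removes the previously stored widget if valid, creates a new one for player controller 0, stores the reference and adds it to the viewport.
; Each event clears only its own widget, so showing one screen leaves the other two untouched.
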(event Custom|CallMainMenuWBP
  (Utilities|IsValid (Variables|Default|GetREF_MainMenu)
    (:Is%20Valid
      (Widget|RemovefromParent (Variables|Default|GetREF_MainMenu)))
    (:Is%20Not%20Valid
      _))
  (bind _returnvalue (UserInterface|CreateWidget "/Game/Blueprints/WBP_MainMenu.WBP_MainMenu_C" (Game|GetPlayerController 0)))
  (bind _output_get (Variables|Default|SetREF_MainMenu _returnvalue))
  (UserInterface|Viewport|AddtoViewport _output_get 0))

(event Custom|CallHUDWBP
  (Utilities|IsValid (Variables|Default|GetREF_HUD)
    (:Is%20Valid
      (Widget|RemovefromParent (Variables|Default|GetREF_HUD)))
    (:Is%20Not%20Valid
      _))
  (bind _returnvalue (UserInterface|CreateWidget "/Game/Blueprints/WBP_HUD.WBP_HUD_C" (Game|GetPlayerController 0)))
  (bind _output_get (Variables|Default|SetREF_HUD _returnvalue))
  (UserInterface|Viewport|AddtoViewport _output_get 0))

(event Custom|CallGameOverWBP
  (Utilities|IsValid (Variables|Default|GetREF_GameOver)
    (:Is%20Valid
      (Widget|RemovefromParent (Variables|Default|GetREF_GameOver)))
    (:Is%20Not%20Valid
      _))
  (bind _returnvalue (UserInterface|CreateWidget "/Game/Blueprints/WBP_GameOver.WBP_GameOver_C" (Game|GetPlayerController 0)))
  (bind _output_get (Variables|Default|SetREF_GameOver _returnvalue))
  (UserInterface|Viewport|AddtoViewport _output_get 0))