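; Wind manager that pushes every Bp_Ball left or right and tilts the PS_Snow_01_Blueprint snow actors to match.
; The Wind Left and Wind Right inputs trigger a gust directly, while the custom Wind event picks a direction at random.
; A Delay-based loop with a shared counter repeatedly adds sideways projectile velocity for about ten seconds, then resets the snow rotation, leaving the added velocity in place.
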(event EventWind
  (if (Math|Random|RandomBool)
    (bind _outactors (Actor|GetAllActorsOfClass "/Game/Blueprints/PS_Snow_01_Blueprint.PS_Snow_01_Blueprint_C"))
    (for _array_element _outactors
      (Transformation|SetActorRotation _array_element "45.000000, 0, 0")
      (Variables|Default|SetTimes 0)
      (Development|PrintString "Let wind pressed" true true "(R=0.536458,G=0.033544,B=0.000000,A=1.000000)")
      (bind _outactors_2 (Actor|GetAllActorsOfClass "/Game/Blueprints/Bp_Ball.Bp_Ball_C" :!label _label))
      (for _array_element_2 _outactors_2
        (Variables|/Script/Engine.MovementComponent|SetVelocity (Variables|/Game/Blueprints/Bp_Ball.Bp_Ball_C|GetProjectileMovement _array_element_2) (+ (Variables|/Script/Engine.MovementComponent|GetVelocity (Variables|/Game/Blueprints/Bp_Ball.Bp_Ball_C|GetProjectileMovement _array_element_2)) "300.000000, 0, 0")))
      (if (== (Variables|Default|GetTimes) 50)
        (Variables|/Script/Engine.MovementComponent|SetVelocity (Variables|/Game/Blueprints/Bp_Ball.Bp_Ball_C|GetProjectileMovement _array_element_2) (Variables|/Script/Engine.MovementComponent|GetVelocity (Variables|/Game/Blueprints/Bp_Ball.Bp_Ball_C|GetProjectileMovement _array_element_2)))
        (bind _outactors_3 (Actor|GetAllActorsOfClass "/Game/Blueprints/PS_Snow_01_Blueprint.PS_Snow_01_Blueprint_C"))
        (for _array_element_3 _outactors_3
          (Transformation|SetActorRotation _array_element_3))
        (else
          (Variables|Default|SetTimes (+ (Variables|Default|GetTimes) 1))
          (Utilities|FlowControl|Delay 0.2)
          (goto _label))))
    (Variables|Default|SetTimes 0)
    (Development|PrintString "Let wind pressed" true true "(R=0.536458,G=0.033544,B=0.000000,A=1.000000)")
    (bind _outactors_4 (Actor|GetAllActorsOfClass "/Game/Blueprints/Bp_Ball.Bp_Ball_C" :!label _label_2))
    (for _array_element_4 _outactors_4
      (Variables|/Script/Engine.MovementComponent|SetVelocity (Variables|/Game/Blueprints/Bp_Ball.Bp_Ball_C|GetProjectileMovement _array_element_4) (+ (Variables|/Script/Engine.MovementComponent|GetVelocity (Variables|/Game/Blueprints/Bp_Ball.Bp_Ball_C|GetProjectileMovement _array_element_4)) "300.000000, 0, 0")))
    (if (== (Variables|Default|GetTimes) 50)
      (Variables|/Script/Engine.MovementComponent|SetVelocity (Variables|/Game/Blueprints/Bp_Ball.Bp_Ball_C|GetProjectileMovement _array_element_4) (Variables|/Script/Engine.MovementComponent|GetVelocity (Variables|/Game/Blueprints/Bp_Ball.Bp_Ball_C|GetProjectileMovement _array_element_4)))
      (bind _outactors_5 (Actor|GetAllActorsOfClass "/Game/Blueprints/PS_Snow_01_Blueprint.PS_Snow_01_Blueprint_C"))
      (for _array_element_5 _outactors_5
        (Transformation|SetActorRotation _array_element_5))
      (else
        (Variables|Default|SetTimes (+ (Variables|Default|GetTimes) 1))
        (Utilities|FlowControl|Delay 0.2)
        (goto _label_2)))
    (else
      (bind _outactors_6 (Actor|GetAllActorsOfClass "/Game/Blueprints/PS_Snow_01_Blueprint.PS_Snow_01_Blueprint_C"))
      (for _array_element_6 _outactors_6
        (Transformation|SetActorRotation _array_element_6 "-45.000000, 0, 0"))
      (Variables|Default|SetTimes 0)
      (Development|PrintString "right wind pressed" true true "(R=0.536458,G=0.033544,B=0.000000,A=1.000000)")
      (bind _outactors_7 (Actor|GetAllActorsOfClass "/Game/Blueprints/Bp_Ball.Bp_Ball_C" :!label _label_3))
      (for _array_element_7 _outactors_7
        (Variables|/Script/Engine.MovementComponent|SetVelocity (Variables|/Game/Blueprints/Bp_Ball.Bp_Ball_C|GetProjectileMovement _array_element_7) (+ (Variables|/Script/Engine.MovementComponent|GetVelocity (Variables|/Game/Blueprints/Bp_Ball.Bp_Ball_C|GetProjectileMovement _array_element_7)) "-300.000000, 0, 0")))
      (if (== (Variables|Default|GetTimes) 50)
        (Variables|/Script/Engine.MovementComponent|SetVelocity (Variables|/Game/Blueprints/Bp_Ball.Bp_Ball_C|GetProjectileMovement _array_element_7) (Variables|/Script/Engine.MovementComponent|GetVelocity (Variables|/Game/Blueprints/Bp_Ball.Bp_Ball_C|GetProjectileMovement _array_element_7)))
        (bind _outactors_8 (Actor|GetAllActorsOfClass "/Game/Blueprints/PS_Snow_01_Blueprint.PS_Snow_01_Blueprint_C"))
        (for _array_element_8 _outactors_8
          (Transformation|SetActorRotation _array_element_8))
        (else
          (Variables|Default|SetTimes (+ (Variables|Default|GetTimes) 1))
          (Utilities|FlowControl|Delay 0.2)
          (goto _label_3))))))

(event Input|ActionEvents|InputActionWindLeft
  (params (Key :type Key%20Structure :default "None"))
  (:Pressed
    (bind _outactors (Actor|GetAllActorsOfClass "/Game/Blueprints/PS_Snow_01_Blueprint.PS_Snow_01_Blueprint_C"))
    (for _array_element _outactors
      (Transformation|SetActorRotation _array_element "45.000000, 0, 0")
      (Variables|Default|SetTimes 0)
      (Development|PrintString "Let wind pressed" true true "(R=0.536458,G=0.033544,B=0.000000,A=1.000000)")
      (bind _outactors_2 (Actor|GetAllActorsOfClass "/Game/Blueprints/Bp_Ball.Bp_Ball_C" :!label _label))
      (for _array_element_2 _outactors_2
        (Variables|/Script/Engine.MovementComponent|SetVelocity (Variables|/Game/Blueprints/Bp_Ball.Bp_Ball_C|GetProjectileMovement _array_element_2) (+ (Variables|/Script/Engine.MovementComponent|GetVelocity (Variables|/Game/Blueprints/Bp_Ball.Bp_Ball_C|GetProjectileMovement _array_element_2)) "300.000000, 0, 0")))
      (if (== (Variables|Default|GetTimes) 50)
        (Variables|/Script/Engine.MovementComponent|SetVelocity (Variables|/Game/Blueprints/Bp_Ball.Bp_Ball_C|GetProjectileMovement _array_element_2) (Variables|/Script/Engine.MovementComponent|GetVelocity (Variables|/Game/Blueprints/Bp_Ball.Bp_Ball_C|GetProjectileMovement _array_element_2)))
        (bind _outactors_3 (Actor|GetAllActorsOfClass "/Game/Blueprints/PS_Snow_01_Blueprint.PS_Snow_01_Blueprint_C"))
        (for _array_element_3 _outactors_3
          (Transformation|SetActorRotation _array_element_3))
        (else
          (Variables|Default|SetTimes (+ (Variables|Default|GetTimes) 1))
          (Utilities|FlowControl|Delay 0.2)
          (goto _label))))
    (Variables|Default|SetTimes 0)
    (Development|PrintString "Let wind pressed" true true "(R=0.536458,G=0.033544,B=0.000000,A=1.000000)")
    (bind _outactors_4 (Actor|GetAllActorsOfClass "/Game/Blueprints/Bp_Ball.Bp_Ball_C" :!label _label_2))
    (for _array_element_4 _outactors_4
      (Variables|/Script/Engine.MovementComponent|SetVelocity (Variables|/Game/Blueprints/Bp_Ball.Bp_Ball_C|GetProjectileMovement _array_element_4) (+ (Variables|/Script/Engine.MovementComponent|GetVelocity (Variables|/Game/Blueprints/Bp_Ball.Bp_Ball_C|GetProjectileMovement _array_element_4)) "300.000000, 0, 0")))
    (if (== (Variables|Default|GetTimes) 50)
      (Variables|/Script/Engine.MovementComponent|SetVelocity (Variables|/Game/Blueprints/Bp_Ball.Bp_Ball_C|GetProjectileMovement _array_element_4) (Variables|/Script/Engine.MovementComponent|GetVelocity (Variables|/Game/Blueprints/Bp_Ball.Bp_Ball_C|GetProjectileMovement _array_element_4)))
      (bind _outactors_5 (Actor|GetAllActorsOfClass "/Game/Blueprints/PS_Snow_01_Blueprint.PS_Snow_01_Blueprint_C"))
      (for _array_element_5 _outactors_5
        (Transformation|SetActorRotation _array_element_5))
      (else
        (Variables|Default|SetTimes (+ (Variables|Default|GetTimes) 1))
        (Utilities|FlowControl|Delay 0.2)
        (goto _label_2)))))

(event Input|ActionEvents|InputActionWindRight
  (params (Key :type Key%20Structure :default "None"))
  (:Pressed
    (bind _outactors (Actor|GetAllActorsOfClass "/Game/Blueprints/PS_Snow_01_Blueprint.PS_Snow_01_Blueprint_C"))
    (for _array_element _outactors
      (Transformation|SetActorRotation _array_element "-45.000000, 0, 0"))
    (Variables|Default|SetTimes 0)
    (Development|PrintString "right wind pressed" true true "(R=0.536458,G=0.033544,B=0.000000,A=1.000000)")
    (bind _outactors_2 (Actor|GetAllActorsOfClass "/Game/Blueprints/Bp_Ball.Bp_Ball_C" :!label _label))
    (for _array_element_2 _outactors_2
      (Variables|/Script/Engine.MovementComponent|SetVelocity (Variables|/Game/Blueprints/Bp_Ball.Bp_Ball_C|GetProjectileMovement _array_element_2) (+ (Variables|/Script/Engine.MovementComponent|GetVelocity (Variables|/Game/Blueprints/Bp_Ball.Bp_Ball_C|GetProjectileMovement _array_element_2)) "-300.000000, 0, 0")))
    (if (== (Variables|Default|GetTimes) 50)
      (Variables|/Script/Engine.MovementComponent|SetVelocity (Variables|/Game/Blueprints/Bp_Ball.Bp_Ball_C|GetProjectileMovement _array_element_2) (Variables|/Script/Engine.MovementComponent|GetVelocity (Variables|/Game/Blueprints/Bp_Ball.Bp_Ball_C|GetProjectileMovement _array_element_2)))
      (bind _outactors_3 (Actor|GetAllActorsOfClass "/Game/Blueprints/PS_Snow_01_Blueprint.PS_Snow_01_Blueprint_C"))
      (for _array_element_3 _outactors_3
        (Transformation|SetActorRotation _array_element_3))
      (else
        (Variables|Default|SetTimes (+ (Variables|Default|GetTimes) 1))
        (Utilities|FlowControl|Delay 0.2)
        (goto _label)))))

(fn ConstructionScript)