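; Patrol enemy character for the block-and-paddle game that is destroyed when the ball hits it.
; On BeginPlay it finds the BP_GM_Block actor and caches its initial and sibling paddles as LowerPaddle and UpperPaddle, which this graph does not use further.
; On Hit it identifies the ball by comparing the class display name to a string rather than casting.
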(event EventBeginPlay
  ;[1 1 1] Get reference of paddles
  (bind _returnvalue (Actor|GetActorOfClass "/Game/Blueprints/BP_GM_Block.BP_GM_Block_C"))
  (Variables|Default|SetlowerPaddle (Variables|/Game/Blueprints/BP_GM_Block.BP_GM_Block_C|GetInitialPaddle _returnvalue))
  (Variables|Default|SetupperPaddle (Variables|/Game/Blueprints/BP_GM_Block.BP_GM_Block_C|GetSiblingPaddle _returnvalue)))

(event Collision|EventHit
  (params (MyComp :type Primitive%20Component%20Object%20Reference) (Other :type Actor%20Object%20Reference) (OtherComp :type Primitive%20Component%20Object%20Reference) (bSelfMoved :type Boolean) (HitLocation :type Vector :default "0, 0, 0") (HitNormal :type Vector :default "0, 0, 0") (NormalImpulse :type Vector :default "0, 0, 0") (Hit :type Hit%20Result%20Structure%20%28by%20ref%29))
  ;[1 1 1] Destroy enemy on ball hit
  (if (Utilities|Enum|Equal(Enum) "Bp_Ball_C" (Utilities|GetClassDisplayName (Utilities|GetClass Other)))
    (Actor|DestroyActor)))

(fn ConstructionScript)