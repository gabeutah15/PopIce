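; BP_Enemy is a patrol AI enemy that provides timeline-driven step and turn movements, with no triggers for them in its own graphs.
; MoveTowardsFaceDirection captures the actor location, then lerps EnemyBody's relative location one DistanceUnit along the body's forward vector, without sweep.
; FaceRotation captures the actor rotation, then lerps EnemyBody's relative rotation by PitchDegreeOffset on pitch rather than yaw.
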(event Custom|MoveTowardsFaceDirection
  (Variables|Default|SetpreviousLocation (Transformation|GetActorLocation))
  (bind _translationlerpvalue (Timeline|TranslationTimeline Play)
    (:Update
      (Transformation|SetRelativeLocation (Variables|Default|GetEnemyBody) (Math|Vector|Lerp(Vector) (Variables|Default|GetpreviousLocation) (+ (Variables|Default|GetpreviousLocation) (* (Math|Vector|GetForwardVector (Variables|Default|GetEnemyBody)) (Variables|Default|GetdistanceUnit))) _translationlerpvalue) false false))))

(event Custom|FaceRotation
  (bind _output_get (Variables|Default|SetpreviousRotation (Transformation|GetActorRotation)))
  (bind _rotatorlerpvalue (Timeline|RotationTimeline Play)
    (:Update
      (Transformation|SetRelativeRotation (Variables|Default|GetEnemyBody) (Math|Rotator|Lerp(Rotator) (Variables|Default|GetpreviousRotation) (Math|Rotator|MakeRotator (.roll _output_get) (+ (.pitch _output_get) (Variables|Default|GetpitchDegreeOffset)) (.yaw _output_get)) _rotatorlerpvalue) false false))))

(event EventBeginPlay)

(fn ConstructionScript)